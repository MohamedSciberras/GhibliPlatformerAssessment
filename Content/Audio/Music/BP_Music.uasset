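; BP_Music is a trigger-box actor that switches area music as the player moves between zones.
; BeginPlay plays a hardcoded opening track on the first BP_Music found in the level.
; Box overlap updates the player's MusicTrack if different, prints it, sets the Audio component's sound, starts it if stopped and sets low volume.
; Leaving mutes instead of stopping; comments mark the switching as unfinished.
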(event `self.ReceiveBeginPlay`
  ;[1 1 1] Only play first area audio on start
  (bind _outactors (`GameplayStatics.GetAllActorsOfClass` "BP_Music_C"))
  (bind _audio (`/Game/Audio/Music/BP_Music.Audio` (`|GetArrayItem` _outactors)))
  (`AudioComponent.SetSound` _audio "/Game/Audio/Music/Path_of_The_Wind_by_Joe_Hisaishi.Path_of_The_Wind_by_Joe_Hisaishi")
  (`AudioComponent.Play` _audio 0.0)
  (`AudioComponent.AdjustVolume` _audio 0.0 0.1 "Linear"))

(event `self.Box.OnComponentBeginOverlap`
  (params (OverlappedComponent :type "PrimitiveComponent Object Reference") (OtherActor :type "Actor Object Reference") (OtherComp :type "PrimitiveComponent Object Reference") (OtherBodyIndex :type Integer) (bFromSweep :type Boolean) (SweepResult :type "HitResult Structure (by ref)"))
  (bind _audio (`self.Audio`))
  (bind _asmy_player_character (cast `/Game/SideScrollerBP/Blueprints/MyPlayerCharacter` OtherActor))
  (if (!= (`self.NewMusicTrack`) (`/Game/SideScrollerBP/Blueprints/MyPlayerCharacter.MusicTrack` _asmy_player_character))
    (bind _output_get (set `/Game/SideScrollerBP/Blueprints/MyPlayerCharacter.MusicTrack` (`self.NewMusicTrack`) _asmy_player_character))
    (`KismetSystemLibrary.PrintString` (`KismetSystemLibrary.GetDisplayName` _output_get))
    ;[1 1 1] bleh needs work
    (`AudioComponent.SetSound` _audio (`self.NewMusicTrack`))
    (switch `EAudioComponentPlayState` (`AudioComponent.GetPlayState` _audio)
      (:`Playing`
        (set `self.IsPlaying` true))
      (:`Stopped`
        (bind _output_get_2 (set `self.IsPlaying` false))))
    (if (not _output_get_2)
      (`AudioComponent.Play` _audio 0.0))
    (`AudioComponent.AdjustVolume` _audio 0.0 0.1 "Linear")))

(event `self.Box.OnComponentEndOverlap`
  (params (OverlappedComponent :type "PrimitiveComponent Object Reference") (OtherActor :type "Actor Object Reference") (OtherComp :type "PrimitiveComponent Object Reference") (OtherBodyIndex :type Integer))
  ;[1 1 1] Reduce Volume to increase on reentry to keep same part of track. Temp stopped to fix ending for overlap switching
  (`AudioComponent.AdjustVolume` (`self.Audio`) 0.0 0.0 "Linear"))

(fn `UserConstructionScript`
  (`AudioComponent.SetSound` (`self.Audio`) (`self.NewMusicTrack`)))