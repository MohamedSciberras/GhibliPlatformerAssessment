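; Game mode that locates the level's BP_MyGameManager and provides creation of the game's UI widgets.
; BeginPlay finds the manager by class and caches it.
; CreateUI spawns the Abandon, Won, Lost, Health and Main widgets, stores each on the manager and adds all to the viewport at once.
; Nothing in this graph calls CreateUI or sets widget visibility.
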(event `self.ReceiveBeginPlay`
  (bind _returnvalue (`GameplayStatics.GetActorOfClass` "/Game/BluePrints/BP_MyGameManager.BP_MyGameManager_C"))
  (set `self.My Game Manager` _returnvalue))

(fn `Create UI`
  (bind _my_game_manager (`/Game/BluePrints/BP_MyFunctionLibrary.Get My Game Manager`))
  (bind _returnvalue (`|CreateWidget` "/Game/UI/Widget_Abandon.Widget_Abandon_C"))
  (bind _output_get (set `/Game/BluePrints/BP_MyGameManager.Widget_Abandon` _returnvalue _my_game_manager))
  (`UserWidget.AddToViewport` _output_get 0)
  (bind _returnvalue_2 (`|CreateWidget` "/Game/UI/Widget_Won.Widget_Won_C"))
  (bind _output_get_2 (set `/Game/BluePrints/BP_MyGameManager.Widget_Won` _returnvalue_2 _my_game_manager))
  (`UserWidget.AddToViewport` _output_get_2 0)
  (bind _returnvalue_3 (`|CreateWidget` "/Game/UI/Widget_Lost.Widget_Lost_C"))
  (bind _output_get_3 (set `/Game/BluePrints/BP_MyGameManager.Widget_Lost` _returnvalue_3 _my_game_manager))
  (`UserWidget.AddToViewport` _output_get_3 0)
  (bind _returnvalue_4 (`|CreateWidget` "/Game/UI/Widget_Health.Widget_Health_C"))
  (bind _output_get_4 (set `/Game/BluePrints/BP_MyGameManager.Widget_Health` _returnvalue_4 _my_game_manager))
  (`UserWidget.AddToViewport` _output_get_4 0)
  (bind _returnvalue_5 (`|CreateWidget` "/Game/UI/Widget_Main.Widget_Main_C"))
  (bind _output_get_5 (set `/Game/BluePrints/BP_MyGameManager.Widget_Main` _returnvalue_5 _my_game_manager))
  (`UserWidget.AddToViewport` _output_get_5 0))

(fn `UserConstructionScript`)