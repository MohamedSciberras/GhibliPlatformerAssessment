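; Cat Bus hazard that shuttles back and forth along a spline via a timeline, with alternating materials as a two-frame, direction-flipped run animation.
; Its damage box knocks the player sideways and up by relative Y position and flickers their mesh.
; A Tick-counted hit timer, reset from the player's HitReset, repeats damage during continuous contact.
; A second trigger briefly forces the player to crouch and prints a dodge message.
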(event `self.ReceiveBeginPlay`
  (`self.StartPlatform`)
  (`PrimitiveComponent.SetMaterial` (`self.ImageHolder`) 0 "/Game/Images/CatBusRun1.CatBusRun1")
  (set `self.CanChangeMaterial` false))

(event `MaterialController`
  ;[1 1 1] Sprite Controller
  (if (not (`self.CanChangeMaterial`))
    (set `self.CanChangeMaterial` true)
    (if (`self.IsFacingLeft`)
      (`PrimitiveComponent.SetMaterial` (`self.ImageHolder`) 0 "/Game/Images/CatBusRun1.CatBusRun1" :!label _label)
      (`KismetSystemLibrary.Delay` 0.5)
      (`PrimitiveComponent.SetMaterial` (`self.ImageHolder`) 0 "/Game/Images/CatBusRun2.CatBusRun2")
      (else
        (`PrimitiveComponent.SetMaterial` (`self.ImageHolder`) 0 "/Game/Images/CatBusRunFlipped1.CatBusRunFlipped1" :!label _label_2)
        (`KismetSystemLibrary.Delay` 0.5)
        (`PrimitiveComponent.SetMaterial` (`self.ImageHolder`) 0 "/Game/Images/CatBusRunFlipped2.CatBusRunFlipped2")))
    (`KismetSystemLibrary.Delay` 0.5)
    (set `self.CanChangeMaterial` false)))

(event `Flicker`
  (params (`My Player` :type "/Game/SideScrollerBP/Blueprints/MyPlayerCharacter Object Reference"))
  (bind _mesh (`Character.Mesh` `My Player`))
  ;[1 1 1] Flicker Visibility based on hit timer based on hit reset in player character
  (`SceneComponent.SetVisibility` _mesh false false :!label _label_3)
  (`KismetSystemLibrary.Delay` 0.2)
  (`SceneComponent.SetVisibility` _mesh true false)
  (`KismetSystemLibrary.Delay` 0.2)
  (if (> (`self.HitTimer`) 0.0)
    (goto _label_3)))

(event `StartPlatform`
  (bind _spline (`self.Spline`))
  ;[1 1 1] Movement
  (bind (_direction _percentofdistance) (`Timeline|SplineTimeline` :!label _label_4)
    (:`Update`
      (`SceneComponent.K2_SetWorldLocation` (`self.StaticMesh`) (`SplineComponent.GetLocationAtDistanceAlongSpline` _spline (* _percentofdistance (`SplineComponent.GetSplineLength` _spline)) "World") false false))
    (:`Finished`
      (`/Engine/EditorBlueprintResources/StandardMacros.FlipFlop`
        (:`A`
          (`self.StartPlatform`)
          (set `self.IsFacingLeft` true)
          (goto _label))
        (:`B`
          (`self.ReversePlatform`)
          (set `self.IsFacingLeft` false)
          (goto _label_2))))))

(event `ReversePlatform`
  ;[1 1 1] Movement
  (goto _label_4 :!via `Reverse`))

(event `self.PlayerDidNotCrouch.OnComponentBeginOverlap`
  (params (OverlappedComponent :type "PrimitiveComponent Object Reference") (OtherActor :type "Actor Object Reference") (OtherComp :type "PrimitiveComponent Object Reference") (OtherBodyIndex :type Integer) (bFromSweep :type Boolean) (SweepResult :type "HitResult Structure (by ref)"))
  ;[1 1 1] Forces Player to crouch underneath
  (bind _asmy_player_character (cast `/Game/SideScrollerBP/Blueprints/MyPlayerCharacter` OtherActor))
  (`Character.Crouch` _asmy_player_character)
  (`KismetSystemLibrary.Delay` 0.2)
  (`Character.UnCrouch` _asmy_player_character)
  (`KismetSystemLibrary.PrintString` "Dodge!!"))

(event `self.Box.OnComponentBeginOverlap`
  (params (OverlappedComponent :type "PrimitiveComponent Object Reference") (OtherActor :type "Actor Object Reference") (OtherComp :type "PrimitiveComponent Object Reference") (OtherBodyIndex :type Integer) (bFromSweep :type Boolean) (SweepResult :type "HitResult Structure (by ref)"))
  (bind _myplayer (`self.MyPlayer`))
  ;[1 1 1] Damager
  (if (`self.ActorHasTag` OtherActor "Tag_Player")
    (bind _asmy_player_character (cast `/Game/SideScrollerBP/Blueprints/MyPlayerCharacter` OtherActor))
    (`self.Knockback` _asmy_player_character)
    (bind _output_get (set `self.MyPlayer` _asmy_player_character))
    (set `self.IsBeingHit` true)
    (if (== (`self.HitTimer`) 0.0)
      (set `self.HitTimer` (`/Game/SideScrollerBP/Blueprints/MyPlayerCharacter.HitReset` _output_get))
      (`self.Flicker` _myplayer)
      (`/Game/SideScrollerBP/Blueprints/MyPlayerCharacter.Change Health` _myplayer -10.0 :!label _label_5)
      (`KismetSystemLibrary.PrintString` (`KismetStringLibrary.Conv_DoubleToString` (`/Game/SideScrollerBP/Blueprints/MyPlayerCharacter.HealthPoints` _myplayer))))))

(event `self.ReceiveTick`
  (params (DeltaSeconds :type "Float (single-precision)"))
  ;[1 1 1] Damager
  (`self.MaterialController`)
  (if (> (`self.HitTimer`) 0.0)
    (bind _result (`/Engine/EditorBlueprintResources/StandardMacros.DecrementFloat` (`self.HitTimer`))
      (:`  `
        (if (and (== _result 0.0) (`self.IsBeingHit`))
          (set `self.HitTimer` (`/Game/SideScrollerBP/Blueprints/MyPlayerCharacter.HitReset` (stale `self.Box.OnComponentBeginOverlap` _output_get)))
          (goto _label_5))))))

(event `self.Box.OnComponentEndOverlap`
  (params (OverlappedComponent :type "PrimitiveComponent Object Reference") (OtherActor :type "Actor Object Reference") (OtherComp :type "PrimitiveComponent Object Reference") (OtherBodyIndex :type Integer))
  ;[1 1 1] this checks continuous contact
  (set `self.IsBeingHit` false))

(event `Knockback`
  (params (`My Player` :type "/Game/SideScrollerBP/Blueprints/MyPlayerCharacter Object Reference"))
  (bind (_returnvalue_x _returnvalue_y) (`KismetMathLibrary.BreakVector` (`SceneComponent.K2_GetComponentLocation` (`self.Box`))))
  (bind (_returnvalue_x_2 _returnvalue_y_2) (`KismetMathLibrary.BreakVector` (`SceneComponent.K2_GetComponentLocation` (`Character.Mesh` `My Player`))))
  ;[1 1 1] Knockback based on comparing world locations
  (if (< _returnvalue_y_2 _returnvalue_y)
    (`Character.LaunchCharacter` `My Player` (0.0 -600.0 600.0) true true)
    (else
      (`Character.LaunchCharacter` `My Player` (0.0 600.0 600.0) true true))))

(fn `UserConstructionScript`)