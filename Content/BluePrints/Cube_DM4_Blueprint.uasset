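; Destructible falling-block Blueprint that resets itself once it has been left alone for a while.
; A Box overlap turns off static rendering on the DestructibleComponent and arms a countdown timer.
; Tick decrements the timer per frame, not by delta time, only while nothing is flagged as overlapping.
; On expiry, AfterOverlapping reassigns the Cube_DM destructible mesh and re-enables static rendering.
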(event `self.ReceiveTick`
  (params (DeltaSeconds :type "Float (single-precision)"))
  ;[1 1 1] Control Falling Blocks with reset after time while not overlapping
  (if (and (not (`self.IsOverlapped`)) (> (`self.Timer`) 0.0))
    (`/Engine/EditorBlueprintResources/StandardMacros.DecrementFloat` (`self.Timer`)
      (:`  `
        (if (<= (`self.Timer`) 0.0)
          (`self.After Overlapping`))))))

(event `self.Box.OnComponentBeginOverlap`
  (params (OverlappedComponent :type "PrimitiveComponent Object Reference") (OtherActor :type "Actor Object Reference") (OtherComp :type "PrimitiveComponent Object Reference") (OtherBodyIndex :type Integer) (bFromSweep :type Boolean) (SweepResult :type "HitResult Structure (by ref)"))
  ;[1 1 1] Control Falling Blocks with reset after time while not overlapping
  (`SkinnedMeshComponent.SetRenderStatic` (`self.DestructibleComponent`) false)
  (set `self.IsOverlapped` true)
  (set `self.Timer` 300.0))

(event `After Overlapping`
  (bind _destructiblecomponent (`self.DestructibleComponent`))
  ;[1 1 1] Control Falling Blocks with reset after time while not overlapping
  (`DestructibleComponent.SetDestructibleMesh` _destructiblecomponent "/Game/BluePrints/Cube_DM.Cube_DM")
  (`SkinnedMeshComponent.SetRenderStatic` _destructiblecomponent true))

(event `self.Box.OnComponentEndOverlap`
  (params (OverlappedComponent :type "PrimitiveComponent Object Reference") (OtherActor :type "Actor Object Reference") (OtherComp :type "PrimitiveComponent Object Reference") (OtherBodyIndex :type Integer))
  ;[1 1 1] Control Falling Blocks with reset after time while not overlapping
  (set `self.IsOverlapped` false))

(fn `UserConstructionScript`)