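; BP_Kiki is a rideable platform that carries its mesh along a spline once a player character holding the platform key enters its box trigger.
; A timeline maps progress to distance along the spline.
; Overlapping a PlayerSpawns actor while riding marks the destination as reached.
; Until then, a player leaving the box sends the platform back after a short delay, unless riding has resumed.
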(event `self.Box.OnComponentBeginOverlap`
  (params (OverlappedComponent :type "PrimitiveComponent Object Reference") (OtherActor :type "Actor Object Reference") (OtherComp :type "PrimitiveComponent Object Reference") (OtherBodyIndex :type Integer) (bFromSweep :type Boolean) (SweepResult :type "HitResult Structure (by ref)"))
  (cast `/Game/BluePrints/PlayerSpawns` OtherActor
    (:`then`
      (if (`self.IsRiding`)
        (set `self.ReachedDestination` true)))
    (:`CastFailed`
      (bind _asmy_player_character (cast `/Game/SideScrollerBP/Blueprints/MyPlayerCharacter` OtherActor))
      (if (`/Game/SideScrollerBP/Blueprints/MyPlayerCharacter.HasPlatformKey` _asmy_player_character)
        (set `self.IsRiding` true)
        (`self.StartPlatform`)))))

(event `StartPlatform`
  (bind _spline (`self.Spline`))
  (bind (_direction _percentofdistance) (`Timeline|SplineTimeline` :!label _label)
    (:`Update`
      (`SceneComponent.K2_SetWorldLocation` (`self.StaticMesh`) (`SplineComponent.GetLocationAtDistanceAlongSpline` _spline (* _percentofdistance (`SplineComponent.GetSplineLength` _spline)) "World") false false))))

(event `ReversePlatform`
  (goto _label :!via `Reverse`))

(event `self.Box.OnComponentEndOverlap`
  (params (OverlappedComponent :type "PrimitiveComponent Object Reference") (OtherActor :type "Actor Object Reference") (OtherComp :type "PrimitiveComponent Object Reference") (OtherBodyIndex :type Integer))
  (cast `/Game/SideScrollerBP/Blueprints/MyPlayerCharacter` OtherActor)
  (if (not (`self.ReachedDestination`))
    (set `self.IsRiding` false)
    (`KismetSystemLibrary.Delay` 1.0)
    (if (not (`self.IsRiding`))
      (`self.ReversePlatform`))))

(fn `UserConstructionScript`)