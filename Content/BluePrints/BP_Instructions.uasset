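; BP_Instructions is a world actor that displays an instructions plane while the player character is nearby.
; The construction script applies the Instructions material to the Plane.
; On BeginPlay the Plane is hidden unless IsVisible is set.
; Box overlap events cast to MyPlayerCharacter, showing the Plane on entry and hiding it on exit, even if it started visible.
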(event `self.ReceiveBeginPlay`
  (`SceneComponent.SetVisibility` (`self.Plane`) false false)
  (if (`self.IsVisible`)
    (`SceneComponent.SetVisibility` (`self.Plane`) true false)))

(event `self.Box.OnComponentBeginOverlap`
  (params (OverlappedComponent :type "PrimitiveComponent Object Reference") (OtherActor :type "Actor Object Reference") (OtherComp :type "PrimitiveComponent Object Reference") (OtherBodyIndex :type Integer) (bFromSweep :type Boolean) (SweepResult :type "HitResult Structure (by ref)"))
  (cast `/Game/SideScrollerBP/Blueprints/MyPlayerCharacter` OtherActor)
  (`SceneComponent.SetVisibility` (`self.Plane`) true false))

(event `self.Box.OnComponentEndOverlap`
  (params (OverlappedComponent :type "PrimitiveComponent Object Reference") (OtherActor :type "Actor Object Reference") (OtherComp :type "PrimitiveComponent Object Reference") (OtherBodyIndex :type Integer))
  (cast `/Game/SideScrollerBP/Blueprints/MyPlayerCharacter` OtherActor)
  (`SceneComponent.SetVisibility` (`self.Plane`) false false))

(fn `UserConstructionScript`
  (`PrimitiveComponent.SetMaterial` (`self.Plane`) 0 (`self.Instructions`)))