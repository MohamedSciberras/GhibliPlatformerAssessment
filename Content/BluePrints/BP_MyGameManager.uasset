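; BP_MyGameManager runs the game flow, switching between main menu, running, won, lost and abandon states.
; Init has the game mode create the UI, initializes the player and enters Main.
; SetState swaps widgets and toggles the mouse, pausing on end states and showing the health HUD while running if applicable.
; ResetGame moves the existing player to a PlayerSpawns actor, indexed by the highest checkpoint number, then re-initializes it.
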(fn `Get State`
  (returns (State :type "/Game/BluePrints/E_MyGameStates Enum"))
  (return (`self.Current Game State`)))

(fn `Init`
  (`KismetSystemLibrary.PrintString` "init")
  (bind _asbp_my_game_mode (cast `/Game/BluePrints/BP_MyGameMode` (`GameplayStatics.GetGameMode`)))
  (`/Game/BluePrints/BP_MyGameMode.Create UI` _asbp_my_game_mode)
  (`/Game/SideScrollerBP/Blueprints/MyPlayerCharacter.Init` (`self.My Player`))
  (`self.Set State` "NewEnumerator5"))

(fn `Reset Game`
  (bind _my_player (`self.My Player`))
  (bind _outactors (`GameplayStatics.GetAllActorsOfClass` "/Game/BluePrints/PlayerSpawns.PlayerSpawns_C"))
  ;[1 1 1] Get Furthest Checkpoint Achieved
  (for _array_element _outactors
    (bind _checkpoint (`/Game/BluePrints/PlayerSpawns.Checkpoint` _array_element))
    (if (> _checkpoint (`self.Largest Checkpoint`))
      (bind _output_get (set `self.Largest Checkpoint` _checkpoint))))
  ;[1 1 1] Respawn Player at PlayerSpawns Location
  (`self.K2_SetActorLocation` _my_player (`self.K2_GetActorLocation` (`|GetArrayItem` _outactors _output_get)) false false)
  (`/Game/SideScrollerBP/Blueprints/MyPlayerCharacter.Init` _my_player))

(fn `Set State`
  (params (`New State` :type "/Game/BluePrints/E_MyGameStates Enum" :default "NewEnumerator0"))
  (if (!= `New State` (`self.Current Game State`))
    (`/Game/BluePrints/BP_MyFunctionLibrary.Hide UI`)
    (bind _output_get (set `self.Current Game State` `New State`))
    (switch `/Game/BluePrints/E_MyGameStates` _output_get
      (:`NewEnumerator0`
        (`/Game/BluePrints/BP_MyFunctionLibrary.Show Mouse` false)
        (`self.Show Hud` true)
        (`GameplayStatics.SetGamePaused` false))
      (:`NewEnumerator1`
        (`GameplayStatics.SetGamePaused` true)
        (`Widget.SetVisibility` (`self.Widget_Won`) "Visible")
        (`/Game/BluePrints/BP_MyFunctionLibrary.Show Mouse` true :!label _label))
      (:`NewEnumerator2`
        (`GameplayStatics.SetGamePaused` true)
        (`Widget.SetVisibility` (`self.Widget_Lost`) "Visible")
        (goto _label))
      (:`NewEnumerator3`
        (`GameplayStatics.SetGamePaused` true)
        (`Widget.SetVisibility` (`self.Widget_Abandon`) "Visible")
        (goto _label))
      (:`NewEnumerator5`
        (`/Game/BluePrints/BP_MyFunctionLibrary.Hide UI`)
        (`Widget.SetVisibility` (`self.Widget_Main`) "Visible")
        (goto _label)))))

(fn `Show Hud`
  (params (Visible :type Boolean))
  (bind _widget_health (`self.Widget_Health`))
  (if Visible
    (if (`/Game/SideScrollerBP/Blueprints/MyPlayerCharacter.HasHealth` (`self.My Player`))
      (`Widget.SetVisibility` _widget_health "Visible"))
    (else
      (`Widget.SetVisibility` _widget_health "Hidden"))))

(fn `UserConstructionScript`)